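; Tutorial trigger volume that shows a message prompt while the third-person player character is inside it.
; On begin overlap it passes its tutorial message to the prompt widget reached through the player's HUD, and on end overlap it hides the prompt.
; An optional show-once flag limits the prompt to the first entry.
; The construction script writes the volume's name into a text component as a label.
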(event OnComponentBeginOverlap(Volume)
  (params (OverlappedComponent :type Primitive%20Component%20Object%20Reference) (OtherActor :type Actor%20Object%20Reference) (OtherComp :type Primitive%20Component%20Object%20Reference) (OtherBodyIndex :type Integer) (bFromSweep :type Boolean) (SweepResult :type Hit%20Result%20Structure%20%28by%20ref%29))
  (bind _asbp_third_person_character (Utilities|Casting|CastToBP_ThirdPersonCharacter OtherActor))
  (if (Variables|Default|GetShowOnce)
    (if (not (Variables|Default|GetHasShown))
      (CallFunction|DisplayTutorial _asbp_third_person_character)
      (Variables|Default|SetHasShown true))
    (else
      (CallFunction|DisplayTutorial _asbp_third_person_character))))

(event OnComponentEndOverlap(Volume)
  (params (OverlappedComponent :type Primitive%20Component%20Object%20Reference) (OtherActor :type Actor%20Object%20Reference) (OtherComp :type Primitive%20Component%20Object%20Reference) (OtherBodyIndex :type Integer))
  (bind _asbp_third_person_character (Utilities|Casting|CastToBP_ThirdPersonCharacter OtherActor))
  (CallFunction|HideTutorial _asbp_third_person_character))

(event EventBeginPlay)

(event Collision|EventActorBeginOverlap
  (params (OtherActor :type Actor%20Object%20Reference)))

(event EventTick
  (params (DeltaSeconds :type Float%20%28single-precision%29)))

(fn ConstructionScript
  (Rendering|Components|TextRender|SetText (Variables|Default|GetTutorial%20Name%20Text) (Variables|Default|GetName)))

(fn DisplayTutorial
  (params (Player :type BP%20Third%20Person%20Character%20Object%20Reference))
  (Default|ShowPrompt (Variables|/Game/GPP/Widgets/WBP_HUD.WBP_HUD_C|GetWBP_TutorialPrompt (Default|GetHUD Player)) (Variables|Default|GetTutorialMessage)))

(fn HideTutorial
  (params (Player :type BP%20Third%20Person%20Character%20Object%20Reference))
  (Default|HidePrompt (Variables|/Game/GPP/Widgets/WBP_HUD.WBP_HUD_C|GetWBP_TutorialPrompt (Default|GetHUD Player))))