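; BP_Door is a door that the third-person character pays chips to open.
; Overlap events track whether the character is nearby and store a reference to it.
; While nearby, each Triggered of the Interact input moves one chip from the character's ChipTotal into the door's paid amount until it reaches OpenCost.
; An Interact press once the cost is met calls Open, which destroys the door actor.
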(event Input|EnhancedActionEvents|EnhancedInputActionIA_Interact
  (params (ActionValue :type Boolean) (ElapsedSeconds :type Float%20%28double-precision%29) (TriggeredSeconds :type Float%20%28double-precision%29) (InputAction :type Input%20Action%20Object%20Reference :default "/Game/GPP/Input/Actions/IA_Interact.IA_Interact"))
  (bind _opencost (Variables|Default|GetOpenCost))
  (:Triggered
    (if (< (Variables|Default|GetChipValuePaid) _opencost)
      (if (Variables|Default|GetPlayerNearby)
        (if (> (Variables|/Game/GPP/Blueprints/BP_ThirdPersonCharacter.BP_ThirdPersonCharacter_C|GetChipTotal (stale Collision|EventActorBeginOverlap _asbp_third_person_character)) 0)
          (Variables|Default|SetChipValuePaid (+ (Variables|Default|GetChipValuePaid) 1))
          (Variables|/Game/GPP/Blueprints/BP_ThirdPersonCharacter.BP_ThirdPersonCharacter_C|SetChipTotal (stale Collision|EventActorBeginOverlap _asbp_third_person_character) (- (Variables|/Game/GPP/Blueprints/BP_ThirdPersonCharacter.BP_ThirdPersonCharacter_C|GetChipTotal (stale Collision|EventActorBeginOverlap _asbp_third_person_character)) 1))))))
  (:Started
    (if (== (Variables|Default|GetChipValuePaid) _opencost)
      (if (Variables|Default|GetPlayerNearby)
        (CallFunction|Open)))))

(event EventBeginPlay)

(event Collision|EventActorBeginOverlap
  (params (OtherActor :type Actor%20Object%20Reference))
  (bind _asbp_third_person_character (Utilities|Casting|CastToBP_ThirdPersonCharacter OtherActor))
  (Variables|Default|SetPlayerNearby true))

(event EventTick
  (params (DeltaSeconds :type Float%20%28single-precision%29)))

(event Collision|EventActorEndOverlap
  (params (OtherActor :type Actor%20Object%20Reference))
  (Utilities|Casting|CastToBP_ThirdPersonCharacter OtherActor)
  (Variables|Default|SetPlayerNearby false))

(fn ConstructionScript)

(fn Open
  (Actor|DestroyActor))