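; BP_Enemy is an enemy actor that holds a hand of cards and displays it through a child-actor hand renderer.
; On BeginPlay it enables player 0 input, constructs a BP_Hand and passes it to the BP_HandRenderer to initialise.
; Pressing 3 adds a random card to the hand and re-renders it.
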(event EventBeginPlay
  (Input|EnableInput (Game|GetPlayerController 0))
  (bind _returnvalue (Game|ConstructObjectfromClass "/Game/GPP/MyStuff/BP_Hand.BP_Hand_C"))
  (bind _output_get (Variables|Default|SetHand _returnvalue))
  ;[0.15 0.15 0.15 0.5] Initialise HandRenderer
  (bind _asbp_hand_renderer (Utilities|Casting|CastToBP_HandRenderer (Variables|/Script/Engine.ChildActorComponent|GetChildActor (Variables|Default|GetBP_HandRenderer))))
  (bind _output_get_2 (Variables|Default|SetHandRenderer _asbp_hand_renderer))
  (Default|InitialiseRenderer _output_get_2 _output_get))

(event Collision|EventActorBeginOverlap
  (params (OtherActor :type Actor%20Object%20Reference)))

(event EventTick
  (params (DeltaSeconds :type Float%20%28single-precision%29)))

(event Input|KeyboardEvents|3
  (params (Key :type Key%20Structure :default "None"))
  (:Pressed
    (Default|AddRandomCard (Variables|Default|GetHand))
    (Default|RenderHand (Variables|Default|GetHandRenderer))))

(fn ConstructionScript)