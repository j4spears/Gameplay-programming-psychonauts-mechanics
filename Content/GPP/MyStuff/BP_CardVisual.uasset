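; BP_CardVisual is the visual representation of a single playing card, showing the sprite that matches its suit and value.
; SetCardData stores the passed card reference, then calls SetCardSprite to refresh the CardSprite.
; SetCardSprite selects one of four per-suit sprite arrays and indexes it by value minus two, so each array starts at the two.
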(event EventBeginPlay)

(event Collision|EventActorBeginOverlap
  (params (OtherActor :type Actor%20Object%20Reference)))

(event EventTick
  (params (DeltaSeconds :type Float%20%28single-precision%29)))

(fn ConstructionScript)

(fn SetCardSprite
  (bind _carddata (Variables|Default|GetCardData))
  (Rendering|Components|Sprite|SetSprite (Variables|Default|GetCardSprite) (Utilities|Array|Get(acopy) (Utilities|Select :Index (Variables|/Game/GPP/MyStuff/BP_Card.BP_Card_C|GetSuit _carddata) :NewEnumerator0 (Variables|Default|GetHeartsSprites) :NewEnumerator1 (Variables|Default|GetClubSprites) :NewEnumerator2 (Variables|Default|GetDiamondsSprites) :NewEnumerator3 (Variables|Default|GetSpadesSprites)) (- (Variables|/Game/GPP/MyStuff/BP_Card.BP_Card_C|GetValue _carddata) 2))))

(fn SetCardData
  (params (CardReference :type BP%20Card%20Object%20Reference))
  (Variables|Default|SetCardData CardReference)
  (CallFunction|SetCardSprite))