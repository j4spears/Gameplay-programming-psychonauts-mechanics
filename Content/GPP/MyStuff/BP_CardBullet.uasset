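; BP_CardBullet is a card projectile actor that either homes in on a target or is released into physics, based on its InitialDeal flag.
; While the flag is true, Tick moves the root toward the Target at constant speed without sweeping and turns it to face that Target.
; Otherwise, Tick enables physics on the Plane and applies a small impulse opposite the actor's forward vector every frame.
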(event EventBeginPlay)

(event Collision|EventActorBeginOverlap
  (params (OtherActor :type Actor%20Object%20Reference)))

(event EventTick
  (params (DeltaSeconds :type Float%20%28single-precision%29))
  (bind _defaultsceneroot (Variables|Default|GetDefaultSceneRoot))
  (bind _target (Variables|Default|GetTarget))
  (bind _plane (Variables|Default|GetPlane))
  (bind _returnvalue (Transformation|GetWorldLocation _defaultsceneroot))
  (bind _rootcomponent (Variables|/Script/Engine.Actor|GetRootComponent _target))
  (bind _returnvalue_2 (Transformation|GetWorldLocation _rootcomponent))
  (if (Variables|Default|GetInitialDeal)
    (Transformation|SetWorldLocation _defaultsceneroot (Math|Interpolation|VInterptoConstant _returnvalue _returnvalue_2 DeltaSeconds 1e+03) false false)
    (Transformation|SetWorldRotation _defaultsceneroot (Math|Rotator|FindLookatRotation _returnvalue _returnvalue_2) false false)
    (else
      (Physics|SetSimulatePhysics _plane true)
      (Physics|AddImpulse _plane (* (Transformation|GetActorForwardVector) -1) "None" false))))

(fn ConstructionScript)