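; BP_Chip is a poker chip pickup that adds its Value to the player's chip total.
; On overlap with a BP_ThirdPersonCharacter, it increases that character's ChipTotal and destroys itself.
; Tick spins the TempPokerChip component by a fixed step each frame, not scaled by delta time.
; An Instantiate function provides a setter for the chip's Value.
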(event EventBeginPlay)

(event Collision|EventActorBeginOverlap
  (params (OtherActor :type Actor%20Object%20Reference))
  (bind _asbp_third_person_character (Utilities|Casting|CastToBP_ThirdPersonCharacter OtherActor))
  (Variables|/Game/GPP/Blueprints/BP_ThirdPersonCharacter.BP_ThirdPersonCharacter_C|SetChipTotal _asbp_third_person_character (+ (Variables|/Game/GPP/Blueprints/BP_ThirdPersonCharacter.BP_ThirdPersonCharacter_C|GetChipTotal _asbp_third_person_character) (Variables|Default|GetValue)))
  (Actor|DestroyActor))

(event EventTick
  (params (DeltaSeconds :type Float%20%28single-precision%29))
  (Transformation|AddLocalRotation (Variables|Default|Gettemp_poker_chip) "0.000000,1.000000,0.000000" false false))

(fn ConstructionScript)

(fn Instantiate
  (params (Value :type Integer))
  (Variables|Default|SetValue Value))