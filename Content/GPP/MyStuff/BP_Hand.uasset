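; BP_Hand represents a hand of cards and tracks the combined value of the cards it holds.
; DrawHand clears the hand and deals two new cards, each constructed as a BP_Card that initialises itself, while AddCard accepts an existing card.
; Every addition calls UpdateTotal, which recomputes the cached Total as a plain sum of card values for GetTotal to return.
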(fn AddCard
  (params (Card :type BP%20Card%20Object%20Reference))
  (Utilities|Array|Add (Variables|Default|GetCards) Card)
  (CallFunction|UpdateTotal))

(fn AddRandomCard
  (bind _returnvalue (Game|ConstructObjectfromClass "/Game/GPP/MyStuff/BP_Card.BP_Card_C"))
  (Default|InitialiseCard _returnvalue)
  (Utilities|Array|Add (Variables|Default|GetCards) _returnvalue)
  (CallFunction|UpdateTotal))

(fn DrawHand
  (Utilities|Array|Clear (Variables|Default|GetCards))
  (CallFunction|AddRandomCard)
  (CallFunction|AddRandomCard))

(fn UpdateTotal
  (Variables|Default|SetTotal 0)
  (for _array_element (Variables|Default|GetCards)
    (Variables|Default|SetTotal (+ (Variables|Default|GetTotal) (Variables|/Game/GPP/MyStuff/BP_Card.BP_Card_C|GetValue _array_element)))))

(fn GetTotal
  (return (Variables|Default|GetTotal)))