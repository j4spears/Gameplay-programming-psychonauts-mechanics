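; BP_Deck is a card deck actor that shoots and deals cards as BP_CardBullet projectiles spawned from its TopCard component.
; It enables player input on BeginPlay, and IA_Shoot fires an untargeted card.
; IA_Deal sends each BP_Enemy an InitialDeal card aimed at it, then passes the deck to that enemy's RecieveSecondCard.
; An unconnected chain for dealing two delayed cards to BP_ThirdPersonCharacter never runs.
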(event Input|EnhancedActionEvents|EnhancedInputActionIA_Deal
  (params (ActionValue :type Boolean) (ElapsedSeconds :type Float%20%28double-precision%29) (TriggeredSeconds :type Float%20%28double-precision%29) (InputAction :type Input%20Action%20Object%20Reference :default "/Game/GPP/Input/Actions/IA_Deal.IA_Deal"))
  (:Started
    (bind _outactors (Actor|GetAllActorsOfClass "/Game/GPP/MyStuff/BP_Enemy.BP_Enemy_C"))
    (for _array_element _outactors
      (CallFunction|DealCard _array_element)
      (Default|RecieveSecondCard _array_element self))))

(event Input|EnhancedActionEvents|EnhancedInputActionIA_Shoot
  (params (ActionValue :type Boolean) (ElapsedSeconds :type Float%20%28double-precision%29) (TriggeredSeconds :type Float%20%28double-precision%29) (InputAction :type Input%20Action%20Object%20Reference :default "/Game/GPP/Input/Actions/IA_Shoot.IA_Shoot"))
  (:Started
    (CallFunction|ShootCard)))

(event EventBeginPlay
  (Input|EnableInput (Game|GetPlayerController 0)))

(event Collision|EventActorBeginOverlap
  (params (OtherActor :type Actor%20Object%20Reference)))

(event EventTick
  (params (DeltaSeconds :type Float%20%28single-precision%29)))

(fn ConstructionScript)

(fn ShootCard
  (bind _topcard (Variables|Default|GetTopCard))
  (bind _returnvalue (Transformation|GetWorldRotation _topcard))
  (bind (_roll _pitch _yaw) (Math|Rotator|BreakRotator _returnvalue))
  (Game|SpawnActorfromClass "/Game/GPP/MyStuff/BP_CardBullet.BP_CardBullet_C" (Math|Transform|MakeTransform (Transformation|GetWorldLocation _topcard) (Math|Rotator|MakeRotator (- _roll 9e+01) _pitch (- _yaw 9e+01))) "AlwaysSpawn" "MultiplyWithRoot" 0 0))

(fn GetTopCardTransform
  (bind _topcard (Variables|Default|GetTopCard))
  (bind _returnvalue (Transformation|GetWorldRotation _topcard))
  (bind (_roll _pitch _yaw) (Math|Rotator|BreakRotator _returnvalue))
  (return (Math|Transform|MakeTransform (Transformation|GetWorldLocation _topcard) (Math|Rotator|MakeRotator (- _roll 9e+01) _pitch (- _yaw 9e+01)))))

(fn DealCard
  (params (Target :type BP%20Enemy%20Object%20Reference))
  (bind _newparam (CallFunction|GetTopCardTransform))
  (bind _returnvalue (Game|SpawnActorfromClass "/Game/GPP/MyStuff/BP_CardBullet.BP_CardBullet_C" _newparam "AlwaysSpawn" "MultiplyWithRoot" 0 0))
  (Variables|/Game/GPP/MyStuff/BP_CardBullet.BP_CardBullet_C|SetInitialDeal _returnvalue true)
  (Variables|/Game/GPP/MyStuff/BP_CardBullet.BP_CardBullet_C|SetTarget _returnvalue Target))