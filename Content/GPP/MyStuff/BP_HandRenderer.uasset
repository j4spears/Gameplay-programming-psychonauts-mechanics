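; BP_HandRenderer is an actor that displays a hand of cards and turns every tick to face the player camera.
; InitialiseRenderer stores the hand reference, and RenderHand destroys and respawns a BP_CardVisual per card, centred along local Y by CardSpacing and attached to the root.
; UpdateCardPositions shifts every rendered card along world Y by the same count-based offset from its current location, rather than laying them out by index.
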(event EventBeginPlay)

(event Collision|EventActorBeginOverlap
  (params (OtherActor :type Actor%20Object%20Reference)))

(event EventTick
  (params (DeltaSeconds :type Float%20%28single-precision%29))
  (Transformation|SetActorRotation (Math|Rotator|FindLookatRotation (Transformation|GetActorLocation) (Camera|GetCameraLocation (Game|GetPlayerCameraManager 0)))))

(fn ConstructionScript)

(fn InitialiseRenderer
  (params (HandReference :type BP%20Hand%20Object%20Reference))
  (Variables|Default|SetHand HandReference))

(fn RenderHand
  (bind _hand (Variables|Default|GetHand))
  (bind _renderedcards (Variables|Default|GetRenderedCards))
  (bind _defaultsceneroot (Variables|Default|GetDefaultSceneRoot))
  (bind _cards (Variables|/Game/GPP/MyStuff/BP_Hand.BP_Hand_C|GetCards _hand))
  (bind _relativelocation (Variables|/Script/Engine.SceneComponent|GetRelativeLocation _defaultsceneroot))
  (bind (_x _y _z) (Math|Vector|BreakVector _relativelocation))
  (for _array_element _renderedcards
    (Actor|DestroyActor _array_element))
  (Utilities|Array|Clear _renderedcards)
  (for (_array_element_2 _array_index) _cards
    (bind _returnvalue (Game|SpawnActorfromClass "/Game/GPP/MyStuff/BP_CardVisual.BP_CardVisual_C" (Math|Conversions|ToTransform(Vector) (Math|Vector|MakeVector _x (+ _y (* (- _array_index (/ (- (Utilities|Array|Length _cards) 1) 2)) (Variables|Default|GetCardSpacing))) _z)) "AlwaysSpawn" "MultiplyWithRoot" 0 0))
    (Default|SetCardData _returnvalue _array_element_2)
    (Transformation|AttachComponentToComponent _returnvalue (Variables|Default|GetDefaultSceneRoot) "None" "KeepRelative" "KeepRelative" "KeepRelative" true)
    (Utilities|Array|Add (Variables|Default|GetRenderedCards) _returnvalue)))

(fn UpdateCardPositions
  (bind _renderedcards (Variables|Default|GetRenderedCards))
  (for _array_element _renderedcards
    (Transformation|SetActorLocation _array_element (Math|Vector|MakeVector (.X (Math|Vector|BreakVector (Transformation|GetActorLocation _array_element))) (+ (.Y (Math|Vector|BreakVector (Transformation|GetActorLocation _array_element))) (* (- 0 (/ (- (Utilities|Array|Length _renderedcards) 1) 2)) (Variables|Default|GetCardSpacing))) (.Z (Math|Vector|BreakVector (Transformation|GetActorLocation _array_element)))) false false)))